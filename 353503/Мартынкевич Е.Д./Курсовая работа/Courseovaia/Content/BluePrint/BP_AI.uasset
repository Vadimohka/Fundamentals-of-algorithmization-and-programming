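; Team-based AI rifle soldier that wanders to random reachable points until it spots an opposing team's pawn.
; PawnSensing filters pawns through BPI_teamInterface, then AIMoveTo closes in and Fire plays a montage and sphere-traces for random damage.
; At zero health it enables mesh physics, hides its bars and reports to GS_TeamDeath.
; Tick updates the health widget and turns both overhead bars toward the player camera.
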(event OnSeePawn(PawnSensing)
  (params (Pawn :type Pawn%20Object%20Reference))
  (if (Utilities|DoesObjectImplementInterface Pawn "/Game/BluePrint/BPI_teamInterface.BPI_teamInterface_C")
    (bind _team (Class|BPITeamInterface|GetTeam(Message) Pawn))
    (if (!= _team (Math|Conversions|ToInteger(Byte) (Variables|Default|GetTeam)))
      (bind _asbp_ai (Utilities|Casting|CastToBP_AI Pawn)
        (:then
          (if (Variables|BP_AI_C|GetisDead? _asbp_ai)
            (CallFunction|SearchAround)
            (else
              (CallFunction|CheseTarget Pawn :!label _label)
              (Variables|Default|SethasSeenTarget true))))
        (:CastFailed
          (goto _label))))))

(event Custom|Search%20Around
  (if (not (Variables|Default|GethasSeenTarget))
    (AI|AIMoveTo self (.RandomLocation (AI|Navigation|GetRandomReachablePointinRadius (Transformation|GetActorLocation) 2e+03 0 0)) 0 3e+02 false
      (:OnSuccess
        (Utilities|FlowControl|Delay 1.0)
        (CallFunction|SearchAround)))))

(event Custom|Chese%20Target
  (params (TargetActor :type Actor%20Object%20Reference))
  (AI|AIMoveTo self "0, 0, 0" TargetActor 4.5e+02 false
    (:OnSuccess
      (CallFunction|Fire TargetActor))))

(event Custom|Fire
  (params (Target%20Actor :type Actor%20Object%20Reference))
  (bind _mesh (Variables|Character|GetMesh))
  (bind _rifle (Variables|Default|GetRifle))
  (bind _returnvalue (Transformation|GetSocketTransform _rifle "b_gun_muzzleflash" "RTS_World"))
  (bind _returnvalue_2 (Transformation|GetWorldRotation _mesh))
  (if (not (Variables|Default|GetisDead?))
    (Pawn|SetControlRotation (Pawn|GetController) (Math|Rotator|FindLookatRotation (Transformation|GetActorLocation) (Transformation|GetActorLocation Target%20Actor)))
    (Animation|Montage|PlayMontage (Variables|Character|GetMesh) "/Game/ShooterAnimations/Idle_Rifle_Shoot_Montage.Idle_Rifle_Shoot_Montage"
      (:then
        (Effects|SpawnEmitterAttached "/Game/InfinityBladeEffects/Effects/FX_Monsters/FX_Monster_Gruntling/Master/P_BackPack_MuzzleFlash.P_BackPack_MuzzleFlash" (Variables|Default|GetRifle) "b_gun_muzzleflash" (.location _returnvalue) _returnvalue_2 "0.150000,0.150000,0.150000" "KeepWorldPosition" true "AutoRelease")
        (Audio|PlaySoundatLocation "/Game/Audio/MS_RifleFire.MS_RifleFire" (Transformation|GetActorLocation) "0, 0, 0" 0.65 1.0 0.0 0 0 0 0)
        (bind (_outhit _returnvalue_3) (Collision|SphereTraceByChannel (.location _returnvalue) (+ (.location _returnvalue) (* (Math|Vector|GetRightVector _returnvalue_2) 3e+03)) 12.0 "TraceTypeQuery1" false 0 "ForDuration"))
        (if _returnvalue_3
          (Game|Damage|ApplyDamage (.HitActor (Collision|BreakHitResult _outhit)) (Math|Random|RandomFloatinRange 3.0 8.0) 0 0)
          (Effects|SpawnEmitteratLocation "/Game/InfinityBladeEffects/Effects/FX_Monsters/FX_Monster_Troll/death/P_TrollDeathImpact.P_TrollDeathImpact" (.ImpactPoint (Collision|BreakHitResult _outhit)) (Math|Rotator|MakeRotfromX (.Normal (Collision|BreakHitResult _outhit))) "0.700000,0.700000,0.700000" true "AutoRelease")
          (Audio|PlaySoundatLocation "/Game/Audio/MS_HitConcrete.MS_HitConcrete" (.ImpactPoint (Collision|BreakHitResult _outhit)) "0, 0, 0" 1.0 1.0 0.0 0 0 0 0))))))

(event EventBeginPlay
  (CallFunction|SearchAround)
  (Utilities|FlowControl|Sequence
    (:then_0
      (if (== (Variables|Default|GetTeam) 1)
        (bind _aswb_ai_team (Utilities|Casting|CastToWB_AI_Team (UserInterface|GetWidget (Variables|Default|GetAI_TeamBar))))
        (Rendering|Components|TextRender|SetText (Variables|/Game/WB_AI_Team.WB_AI_Team_C|Getteam_text _aswb_ai_team) "Team B")))
    (:then_1
      (Utilities|FlowControl|Delay 0.3 :!label _label)
      (if (Variables|Default|GethasSeenTarget)
        (CallFunction|SearchAround)
        (Variables|Default|SethasSeenTarget false)
        (goto _label)))))

(event EventTick
  (params (DeltaSeconds :type Float%20%28single-precision%29))
  (bind _aswb_ai_health_hud (Utilities|Casting|CastToWB_AI_HealthHUD (UserInterface|GetWidget (Variables|Default|GetAI_HealthBar))))
  (Progress|SetPercent (Variables|/Game/WB_AI_HealthHUD.WB_AI_HealthHUD_C|GetHealthBar _aswb_ai_health_hud) (/ (Variables|Default|GetHealth) 1e+02))
  (Transformation|SetWorldRotation (Variables|Default|GetAI_HealthBar) (Math|Rotator|FindLookatRotation (Transformation|GetActorLocation) (Transformation|GetActorLocation (Game|GetPlayerCameraManager 0))) false false))

(event EventSetTeam
  (params (team :type E_Teams%20Enum :default "NewEnumerator0"))
  (Variables|Default|SetTeam team))

(event Game|Damage|EventAnyDamage
  (params (Damage :type Float%20%28single-precision%29) (DamageType :type Damage%20Type%20Object%20Reference) (InstigatedBy :type Controller%20Object%20Reference) (DamageCauser :type Actor%20Object%20Reference))
  (Variables|Default|SetHealth (- (Variables|Default|GetHealth) Damage))
  (if (<= (Variables|Default|GetHealth) 0.0)
    (Development|PrintString "Die")
    (Physics|SetSimulatePhysics (Variables|Character|GetMesh) true)
    (Pawn|Components|CharacterMovement|SetMovementMode (Variables|Character|GetCharacterMovement) "MOVE_None" 0)
    (Variables|Default|SetisDead? true)
    (Rendering|SetVisibility (Variables|Default|GetAI_HealthBar) false false)
    (bind _asgs_team_death (Utilities|Casting|CastToGS_TeamDeath (Game|GetGameState)))
    (Default|DecreaseTeamNumbers _asgs_team_death (== (Variables|Default|GetTeam) 0))
    (else
      (Development|PrintString "Damage"))))

(fn ConstructionScript)

(fn GetTeam
  (return (Variables|Default|GetTeam)))