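; Game State, by its GS prefix, for a team elimination mode, meant to track living players on Team A and Team B.
; DecreaseTeamnumbers takes a team flag, sets that team's alive count and prints the opposing team as winner at zero or below.
; The decrement nodes feeding those counts sit off the execution path, and an unconnected SetGamePaused node means a win only prints a message.
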(event Custom|Decrease%20Team%20numbers
  (params (Team%20A :type Boolean))
  (if Team%20A
    (bind _output_get (Variables|Default|SetnumberOfTeamA_Alive (stale _result)))
    (if (<= _output_get 0)
      (Development|PrintString "TEAM B WON"))
    (else
      (bind _output_get_2 (Variables|Default|SetnumberOfTeamB_Alive (stale _result)))
      (if (<= _output_get_2 0)
        (Development|PrintString "TEAM A WON")))))

(fn ConstructionScript)